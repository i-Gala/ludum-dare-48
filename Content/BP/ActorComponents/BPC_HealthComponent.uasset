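; Actor component that gives its owner health, damage handling and death.
; Health starts at the maximum on BeginPlay, and ReceiveHit subtracts damage only while Damageable is set, firing the DamageReceived dispatcher before the subtraction.
; At zero or below it calls KillActor, which fires ActorKilled and destroys the owner immediately, or through a lifespan when given a positive delay.
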(event `self.ReceiveBeginPlay`
  (set `self.CurrentHealth` (`self.MaxHealth`)))

(fn `KillActor`
  (params (Delay :type "Float (double-precision)"))
  (bind _returnvalue (`self.GetOwner`))
  (`/Engine/EditorBlueprintResources/StandardMacros.IsValid` _returnvalue
    (:`Is Valid`
      (`self.ActorKilled`)
      (if (> (`local.Delay`) 0.0)
        (`Actor.SetLifeSpan` _returnvalue (`local.Delay`))
        (else
          (`Actor.K2_DestroyActor` _returnvalue))))))

(fn `ReceiveHit`
  (params (Damage :type Integer))
  (if (`self.bDamageable`)
    (`self.DamageReceived`)
    (bind _output_get (set `self.CurrentHealth` (- (`self.CurrentHealth`) (`local.Damage`))))
    (if (<= _output_get 0)
      (`self.KillActor` 0.0))))