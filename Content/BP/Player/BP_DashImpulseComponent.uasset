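; Player component that gives BP_Player a directional dash with an optional charged version, plus particles and sounds.
; StartCharging lowers walk speed, starts charge effects and enables Tick to accumulate charge time while the player can move.
; Execute launches the character with normal or charged impulse, falling back to forward when horizontal input is near zero and damping vertical velocity.
; DashBoxComponent collision is enabled during the dash, then a cooldown gates the next one.
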(event `self.ReceiveBeginPlay`
  (bind _asbp_player (cast `/Game/BP/Player/BP_Player` (`self.GetOwner`)))
  (set `self.BP_Player` _asbp_player))

(event `Execute`
  (params (Direction :type "Vector Structure") (IsCharged :type Boolean))
  (bind (_direction_x _direction_y _direction_z) (`KismetMathLibrary.BreakVector` (`self.Direction`)))
  (bind (_direction_x_2 _direction_y_2 _direction_z_2) (`KismetMathLibrary.BreakVector` (`self.Direction`)))
  (bind _returnvalue (`KismetMathLibrary.SelectFloat` (`self.ChargedDashImpulse`) (`self.DashImpulse`) (`self.bIsCharging`)))
  (bind (_returnvalue_x _returnvalue_y) (`KismetMathLibrary.BreakVector` (select `bool` (== (`KismetMathLibrary.Conv_VectorToVector2D` (`self.Direction`)) (0.0 0.0) :`ErrorTolerance` 0.2) :`false` (`self.Direction`) :`true` (`Actor.GetActorForwardVector` (`self.BP_Player`)))))
  (bind (_returnvalue_x_2 _returnvalue_y_2) (`KismetMathLibrary.BreakVector` (* (`KismetMathLibrary.MakeVector` _returnvalue_x _returnvalue_y _direction_z_2) _returnvalue)))
  (`self.SetComponentTickEnabled` false)
  (set `self.bIsCharging` (>= (`self.ChargingTimeCurrent`) (`self.ChargingTime`)))
  (set `self.ChargingTimeCurrent` 0.0)
  (set `self.Direction` Direction)
  (if (and (`self.bCanDash`) (`/Game/BP/Player/BP_Player.FCanMove` (`self.BP_Player`)))
    (set `self.bIsDashing` true)
    (set `self.bCanDash` false)
    (set `CharacterMovementComponent.MaxWalkSpeed` (`self.CharacterBaseSpeed`) (`Character.CharacterMovement` (`self.BP_Player`)))
    (`self.SpawnParticle`)
    (`GameplayStatics.SpawnSound2D` "/Game/Sound/dash_Cue.dash_Cue" 1.0 1.0 0.0 null)
    (`GameplayStatics.SpawnSound2D` "/Game/Sound/quack1_Cue.quack1_Cue" 1.0 1.0 0.0 null)
    (`MovementComponent.StopMovementImmediately` (`Character.CharacterMovement` (`self.BP_Player`)))
    (`self.EnableCollision` true)
    (`Character.LaunchCharacter` (`self.BP_Player`) (`KismetMathLibrary.MakeVector` _returnvalue_x_2 _returnvalue_y_2 (`KismetMathLibrary.SelectFloat` 0.0 (`KismetMathLibrary.SelectFloat` (* (/ _returnvalue 4.0) _direction_z) (* (/ _returnvalue 8.0) _direction_z) (> _direction_z 0.0)) (== _direction_z 0.0))) true true)
    (`KismetSystemLibrary.Delay` (`self.DashDuration`))
    (`MovementComponent.StopMovementImmediately` (`Character.CharacterMovement` (`self.BP_Player`)))
    (`self.EnableCollision` false)
    (set `self.bIsDashing` false)
    (`KismetSystemLibrary.Delay` (`self.Cooldown`))
    (set `self.bIsCharging` false)
    (set `self.bCanDash` true)
    (else
      (set `self.bIsCharging` false))))

(event `EnableCollision`
  (params (Enable :type Boolean))
  (if Enable
    (`PrimitiveComponent.SetCollisionEnabled` (`/Game/BP/Player/BP_Player.DashBoxComponent` (`self.BP_Player`)) "QueryAndPhysics")
    (else
      (`PrimitiveComponent.SetCollisionEnabled` (`/Game/BP/Player/BP_Player.DashBoxComponent` (`self.BP_Player`)) "NoCollision"))))

(event `SpawnParticle`
  ;[0.2159 0.8714 1 0.5529] VFX
  (bind _chargingps (`self.ChargingPS`)
    (:`then`
      (`self.Deactivate` _chargingps))
    (:`else`
      _))
  (bind _dashparticle (`self.DashParticle`)
    (:`then`
      (`self.Activate` _dashparticle true))
    (:`else`
      (bind _returnvalue (`GameplayStatics.SpawnEmitterAttached` "/Game/Materials/PS_Dash.PS_Dash" (`Actor.RootComponent` (`self.BP_Player`)) "None" (0.0 0.0 0.0) (struct) (1.0 1.0 1.0) "SnapToTarget"))))
  (bind _output_get (set `self.DashParticle` _returnvalue))
  (`KismetSystemLibrary.Delay` (+ (`self.DashDuration`) 0.1))
  (`self.Deactivate` _output_get)
  (bind _chargeend (`self.ChargeEnd`)
    (:`then`
      (`self.Deactivate` _chargeend))
    (:`else`)))

(event `StartCharging`
  (bind _bcandash (`self.bCanDash`))
  ;[0.2159 0.8714 1 0.5529] Charging
  (if (`self.bIsCharging`)
    (if (`self.bCanDash`)
      (`self.SetComponentTickEnabled` false))
    (else
      (set `self.ChargingTimeCurrent` 0.0)
      (set `self.bIsCharging` _bcandash)
      (`self.SetComponentTickEnabled` _bcandash)
      (if _bcandash
        (set `CharacterMovementComponent.MaxWalkSpeed` (`self.ChargingWalkSpeed`) (`Character.CharacterMovement` (`self.BP_Player`)))
        (bind _returnvalue (`GameplayStatics.SpawnEmitterAttached` "/Game/Materials/PS_Charge.PS_Charge" (`Actor.RootComponent` (`self.BP_Player`)) "None" (0.0 0.0 0.0) (struct) (1.0 1.0 1.0) "SnapToTarget"))
        (set `self.ChargingPS` _returnvalue)
        (`/Engine/EditorBlueprintResources/StandardMacros.DoOnce` false :!label _label
          (:`Completed`
            (bind _returnvalue_2 (`GameplayStatics.SpawnEmitterAttached` "/Game/Materials/PS_ChargeEnd.PS_ChargeEnd" (`Actor.RootComponent` (`self.BP_Player`)) "None" (0.0 0.0 0.0) (struct) (1.0 1.0 1.0) "SnapToTarget"))
            (set `self.ChargeEnd` _returnvalue_2)
            (`KismetSystemLibrary.Delay` 0.2)
            (`self.Deactivate` _returnvalue_2)))))))

(event `ChargingStop`
  ;[0.2159 0.8714 1 0.5529] Charging
  (`self.SetComponentTickEnabled` false)
  (set `self.bIsCharging` false))

(event `self.ReceiveTick`
  (params (DeltaSeconds :type "Float (single-precision)"))
  ;[0.2159 0.8714 1 0.5529] Charging
  (if (`/Game/BP/Player/BP_Player.FCanMove` (`self.BP_Player`))
    (bind _output_get (set `self.ChargingTimeCurrent` (+ (`self.ChargingTimeCurrent`) DeltaSeconds)))
    (if (>= _output_get (`self.ChargingTime`))
      (goto _label))
    (else
      (set `self.ChargingTimeCurrent` 0.0)
      (goto _label :!via `Reset`))))