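; BP_CameraPlayer is a camera actor that moves continuously along its camera's forward vector while a Player reference is valid.
; Tick offsets the actor by a frame-rate-independent step, without sweep, and skips the move when speed is zero.
; GetSpeed switches from Speed to SpeedRelocate when the distance to the Player exceeds DistanceMax.
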(event `self.ReceiveTick`
  (params (DeltaSeconds :type "Float (single-precision)"))
  (`self.Player`
    (:`then`
      (bind _speed (`self.GetSpeed`))
      (if (!= _speed 0.0)
        (`self.K2_SetActorLocation` (+ (`self.K2_GetActorLocation`) (* (`SceneComponent.GetForwardVector` (`self.CameraComponent`)) (* _speed DeltaSeconds))))))
    (:`else`)))

(fn `GetSpeed`
  (returns (speed :type "Float (double-precision)"))
  (return (`KismetMathLibrary.SelectFloat` (`self.SpeedRelocate`) (`self.Speed`) (> (`self.GetDistanceTo` (`self.Player`) self) (`self.DistanceMax`)))))

(fn `UserConstructionScript`)