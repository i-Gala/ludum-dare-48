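; Player component that scores how many steps BP_Player has descended and calls game over when a fall is too deep.
; It caches the starting height on BeginPlay, destroying itself if the owner is not a BP_Player.
; While walking, Tick converts the height drop into whole steps as the score.
; When not walking, it records the fall's starting height and fires OnGameOver once the drop exceeds the StepFall limit.
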(event `self.ReceiveBeginPlay`
  (bind _asbp_player (cast `/Game/BP/Player/BP_Player` (`self.GetOwner`))
    (:`then`
      (bind _output_get (set `self.Player` _asbp_player))
      (bind (_returnvalue_x _returnvalue_y _returnvalue_z) (`KismetMathLibrary.BreakVector` (`Actor.K2_GetActorLocation` _output_get)))
      (set `self.ZOriginal` _returnvalue_z))
    (:`CastFailed`
      (`self.K2_DestroyComponent`))))

(event `self.ReceiveTick`
  (params (DeltaSeconds :type "Float (single-precision)"))
  (bind _player (`self.Player`)
    (:`then`
      (if (`CharacterMovementComponent.IsWalking` (`Character.CharacterMovement` _player))
        (if (`self.bIsFalling`)
          (set `self.bIsFalling` false)
          (else
            (bind (_returnvalue_x _returnvalue_y _returnvalue_z) (`KismetMathLibrary.BreakVector` (`Actor.K2_GetActorLocation` _player)))
            (set `self.Score` (`KismetMathLibrary.FTrunc` (/ (- (`self.ZOriginal`) _returnvalue_z) (`self.StepHeight`))))))
        (elif (`self.bIsFalling`)
          (if (> (/ (- (`self.ZFall`) _returnvalue_z) (`self.StepHeight`)) (`self.StepFall`))
            (`self.OnGameOver`))
          (else
            (set `self.bIsFalling` true)
            (set `self.ZFall` _returnvalue_z)))))
    (:`else`)))