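; Actor component that gives BP_Player a timed dash in a supplied input direction.
; Execute raises max and min analog walk speed to dash speed, enables query collision on the player's DashBoxComponent and turns on tick.
; Tick forces movement input until time runs out, then stops walking movement, restores speeds and collision, and starts a cooldown timer.
; Execute itself does not check the cooldown flag.
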(event `self.ReceiveBeginPlay`
  (bind _asbp_player (cast `/Game/BP/Player/BP_Player` (`self.GetOwner`)))
  (set `self.As BP Player` _asbp_player)
  (bind _charactermovement (`Character.CharacterMovement` _asbp_player))
  (set `self.WalkOriginal` (`CharacterMovementComponent.MaxWalkSpeed` _charactermovement))
  (set `self.WalkMinOriginal` (`CharacterMovementComponent.MinAnalogWalkSpeed` _charactermovement)))

(event `Execute`
  (params (InputVector :type "Vector Structure"))
  (bind _as_bp_player (`self.As BP Player`))
  (bind _charactermovement (`Character.CharacterMovement` _as_bp_player))
  (set `self.Input Vector` InputVector)
  (set `self.currentTime` 0.0)
  (set `self.bIsDashing` true)
  (set `CharacterMovementComponent.MaxWalkSpeed` (`self.speed`) _charactermovement)
  (set `CharacterMovementComponent.MinAnalogWalkSpeed` (`self.speed`) _charactermovement)
  (`PrimitiveComponent.SetCollisionEnabled` (`/Game/BP/Player/BP_Player.DashBoxComponent` _as_bp_player) "QueryOnly")
  (`self.SetComponentTickEnabled` true))

(event `self.ReceiveTick`
  (params (DeltaSeconds :type "Float (single-precision)"))
  (bind _as_bp_player (`self.As BP Player`))
  (bind _charactermovement (`Character.CharacterMovement` _as_bp_player))
  (if true
    (`Pawn.AddMovementInput` _as_bp_player (`self.Input Vector`) 1.0 true)
    (bind _output_get (set `self.currentTime` (+ DeltaSeconds (`self.currentTime`))))
    (if (>= _output_get (`self.time`))
      (`self.SetComponentTickEnabled` false)
      (if (`CharacterMovementComponent.IsWalking` _charactermovement)
        (`MovementComponent.StopMovementImmediately` _charactermovement))
      (set `self.bIsDashing` false)
      (set `self.bCooldown` true)
      (`PrimitiveComponent.SetCollisionEnabled` (`/Game/BP/Player/BP_Player.DashBoxComponent` _as_bp_player) "NoCollision")
      (set `CharacterMovementComponent.MaxWalkSpeed` (`self.WalkOriginal`) _charactermovement)
      (set `CharacterMovementComponent.MinAnalogWalkSpeed` (`self.WalkMinOriginal`) _charactermovement)
      (bind _returnvalue (`KismetSystemLibrary.K2_SetTimerDelegate` (delegate `CooldownEnd`) (`self.Cooldown`)))
      (set `self.CooldownTimer` _returnvalue))))

(event `CooldownEnd`
  (set `self.bCooldown` false)
  (`KismetSystemLibrary.K2_ClearAndInvalidateTimerHandle` (`self.CooldownTimer`)))