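; Player character Blueprint with world-axis movement, an impulse dash and a separate camera actor set as view target.
; Move and dash inputs check CanMove, and dash direction comes from the movement axes.
; The dash box's overlap damages obstacles through their health component.
; Tick drives reused step and landing particles; GameOver is empty, health events only print, and the older dash component call is disconnected.
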(event `self.ReceiveBeginPlay`
  (bind _camera (`self.Camera`)
    (:`then`
      (`/Game/BP/Player/BP_CameraPlayer.UpdatePlayer` _camera self)
      (`PlayerController.SetViewTargetWithBlend` (`GameplayStatics.GetPlayerController` 0) _camera 0.0 "VTBlend_Linear" 0.0 false)
      (add `/Game/BP/Player/BP_ScoreComponent.OnGameOver` (`self.BP_ScoreComponent`) (`|CreateDelegate` :!event `Game Over`)))
    (:`else`)))

(event `InputAxis|MoveRight`
  (params (AxisValue :type "Float (single-precision)"))
  ;[0.9387 0 1 0.1373] Movement
  (if (`self.CanMove`)
    (`self.AddMovementInput` (0.0 1.0 0.0) AxisValue)))

(event `Game Over`
  ;[0.9387 0 1 0.1373] Game Over
)

(event `InputAxis|MoveForward`
  (params (AxisValue :type "Float (single-precision)"))
  ;[0.9387 0 1 0.1373] Movement
  (if (`self.CanMove`)
    (`self.AddMovementInput` (1.0 0.0 0.0) AxisValue)))

(event `InputAction|Dash`
  (params (Key :type "Key Structure"))
  ;[0.9387 0 1 0.1373] Dash
  (:`Released`
    (if (`self.CanMove`)
      (`/Game/BP/Player/BP_DashImpulseComponent.Execute` (`self.BP_DashImpulseComponent`) (`KismetMathLibrary.MakeVector` (`self.GetInputAxisValue`) (`self.GetInputAxisValue`)) false))))

(event `self.DashBoxComponent.OnComponentBeginOverlap`
  (params (OverlappedComponent :type "PrimitiveComponent Object Reference") (OtherActor :type "Actor Object Reference") (OtherComp :type "PrimitiveComponent Object Reference") (OtherBodyIndex :type Integer) (bFromSweep :type Boolean) (SweepResult :type "HitResult Structure (by ref)"))
  ;[0.9387 0 1 0.1373] Dash
  ;;[0.9693 0.5 1 0.48] Dashea contra objetos
  (bind _asbp_obstacle_base (cast `/Game/BP/Obstacles/BP_ObstacleBase` OtherActor))
  (`/Game/BP/ActorComponents/BPC_HealthComponent.ReceiveHit` (`/Game/BP/Obstacles/BP_ObstacleBase.BPC_HealthComponent` _asbp_obstacle_base) (`/Game/BP/Player/BP_DashComponent.Damage` (`self.BP_DashComponent`))))

(event `self.BPC_HealthComponent.DamageReceived`
  (`KismetSystemLibrary.PrintString` "DamageReceived"))

(event `self.BPC_HealthComponent.ActorKilled`
  (`KismetSystemLibrary.PrintString` "Dead - Game Over"))

(event `self.ReceiveTick`
  (params (DeltaSeconds :type "Float (single-precision)"))
  (`|ExecutionSequence`
    (:`then_0`
      (bind _output_get (set `self.MoventParticleTimer` (+ DeltaSeconds (`self.MoventParticleTimer`))))
      (if (> _output_get (`self.MovementParticleCooldown`))
        (if (`self.CanSpawnWalkParticle`)
          (set `self.MoventParticleTimer` 0.0)
          (`self.SpawnStepParticle`))))
    (:`then_1`
      (if (`NavMovementComponent.IsFalling` (`self.CharacterMovement`))
        (set `self.HaveToLand` true)
        (elif (`self.HaveToLand`)
          (set `self.HaveToLand` false)
          (`self.SpawnLandParticle`))))))

(event `SpawnStepParticle`
  (bind _stepparticle (`self.StepParticle`)
    (:`then`
      (`ActorComponent.Activate` _stepparticle true))
    (:`else`
      (bind _returnvalue (`GameplayStatics.SpawnEmitterAttached` "/Game/Materials/PS_Run.PS_Run" (`self.CapsuleComponent`) "None" (0.0 0.0 0.0) (struct) (1.0 1.0 1.0) "SnapToTarget"))))
  (bind _output_get (set `self.StepParticle` _returnvalue))
  (`KismetSystemLibrary.Delay` 0.2)
  (`ActorComponent.Deactivate` _output_get))

(event `SpawnLandParticle`
  (bind _landparticle (`self.LandParticle`)
    (:`then`
      (`ActorComponent.Activate` _landparticle true))
    (:`else`
      (bind _returnvalue (`GameplayStatics.SpawnEmitterAttached` "/Game/Materials/PS_Land.PS_Land" (`self.CapsuleComponent`) "None" (0.0 0.0 0.0) (struct) (1.0 1.0 1.0) "SnapToTarget"))))
  (bind _output_get (set `self.LandParticle` _returnvalue))
  (`KismetSystemLibrary.Delay` 0.2)
  (`ActorComponent.Deactivate` _output_get))

(fn `CanSpawnWalkParticle`
  (returns (ReturnValue :type Boolean))
  (bind _charactermovement (`self.CharacterMovement`))
  (return (and (`CharacterMovementComponent.IsWalking` _charactermovement) (> (`KismetMathLibrary.VSize` (`MovementComponent.Velocity` _charactermovement)) 0.0))))

(fn `UserConstructionScript`)