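; Enemy obstacle that periodically damages the player nearby and knocks them back on contact.
; A looping timer is started on BeginPlay, and the Attack event runs a debug-drawn sphere trace at the actor's location, damaging a hit BP_Player through its health component.
; Hitting the static mesh stops the player's movement and applies a horizontal velocity impulse opposite the player's facing, rather than away from the enemy.
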(event `self.ReceiveBeginPlay`
  (bind _returnvalue (`KismetSystemLibrary.K2_SetTimerDelegate` (`|CreateDelegate` :!event `Attack`) (`self.TimeBetweenAttack`) true))
  (set `self.TimerHandle` _returnvalue))

(event `Attack`
  (bind _returnvalue (`self.K2_GetActorLocation`))
  (bind _outhit (`KismetSystemLibrary.SphereTraceSingleForObjects` :`Start` _returnvalue :`End` _returnvalue :`Radius` (`self.AttackRadius`) :`ObjectTypes` (`self.Object Types`) :`DrawDebugType` "ForDuration"))
  (bind _asbp_player (cast `/Game/BP/Player/BP_Player` (`.HitActor` (`GameplayStatics.BreakHitResult` _outhit))))
  (`/Game/BP/ActorComponents/BPC_HealthComponent.ReceiveHit` (`/Game/BP/Player/BP_Player.BPC_HealthComponent` _asbp_player) (`self.DamageToDeal`)))

(event `self.StaticMesh.OnComponentHit`
  (params (HitComponent :type "PrimitiveComponent Object Reference") (OtherActor :type "Actor Object Reference") (OtherComp :type "PrimitiveComponent Object Reference") (NormalImpulse :type "Vector Structure") (Hit :type "HitResult Structure (by ref)"))
  ;[1 1 1] Apply impulse on player if they hit the Static Mesh
  (bind _asbp_player (cast `/Game/BP/Player/BP_Player` OtherActor))
  (bind _charactermovement (`Character.CharacterMovement` _asbp_player))
  (`MovementComponent.StopMovementImmediately` _charactermovement)
  (bind (_returnvalue_x _returnvalue_y) (`KismetMathLibrary.BreakVector` (* (* (`self.GetActorForwardVector` _asbp_player) -1.0) 1000.0)))
  (`CharacterMovementComponent.AddImpulse` _charactermovement (`KismetMathLibrary.MakeVector` _returnvalue_x _returnvalue_y) true))

(fn `UserConstructionScript`
  (`parent.UserConstructionScript`))