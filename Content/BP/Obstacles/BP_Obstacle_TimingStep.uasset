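; BP_Obstacle_TimingStep is an obstacle step that blinks between hidden and visible on a fixed timer.
; BeginPlay starts a looping timer at TimeToDisappear, apparently driving SwitchState, whose FlipFlop alternately calls EnableStep with false and true, starting hidden.
; EnableStep toggles StaticMesh visibility, but both branches set collision to QueryAndPhysics, so the hidden step stays solid.
; EndPlay clears the timer.
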(event `self.ReceiveBeginPlay`
  (bind _returnvalue (`KismetSystemLibrary.K2_SetTimerDelegate` (`|CreateDelegate` :!event `SwitchState`) (`self.TimeTo Disappear`) true))
  (set `self.TimerHandle` _returnvalue))

(event `SwitchState`
  (`/Engine/EditorBlueprintResources/StandardMacros.FlipFlop`
    (:`A`
      (`self.EnableStep` false))
    (:`B`
      (`self.EnableStep` true))))

(event `self.ReceiveEndPlay`
  (params (EndPlayReason :type "EEndPlayReason Enum" :default "Destroyed"))
  (`KismetSystemLibrary.K2_ClearAndInvalidateTimerHandle` (`self.TimerHandle`)))

(fn `EnableStep`
  (params (Enable :type Boolean))
  (bind _staticmesh (`self.StaticMesh`))
  (if Enable
    (`PrimitiveComponent.SetCollisionEnabled` _staticmesh "QueryAndPhysics")
    (`SceneComponent.SetVisibility` (`self.StaticMesh`) (`local.Enable`) false)
    (else
      (`PrimitiveComponent.SetCollisionEnabled` _staticmesh "QueryAndPhysics")
      (`SceneComponent.SetVisibility` (`self.StaticMesh`) (`local.Enable`) false)))
  (return))

(fn `UserConstructionScript`
  (`parent.UserConstructionScript`))