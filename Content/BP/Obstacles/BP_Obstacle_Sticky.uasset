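; BP_Obstacle_Sticky is an obstacle that changes the player's walk speed while they overlap its Box.
; When the player's capsule enters, it caches the current max speed in SpeedOriginal, halts movement unless the player is dashing, and sets MaxWalkSpeed to SpeedMax.
; When the capsule leaves, it restores MaxWalkSpeed from that cached value, which is stored on the obstacle itself.
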(event `self.Box.OnComponentBeginOverlap`
  (params (OverlappedComponent :type "PrimitiveComponent Object Reference") (OtherActor :type "Actor Object Reference") (OtherComp :type "PrimitiveComponent Object Reference") (OtherBodyIndex :type Integer) (bFromSweep :type Boolean) (SweepResult :type "HitResult Structure (by ref)"))
  (bind _asbp_player (cast `/Game/BP/Player/BP_Player` OtherActor))
  (`/Engine/EditorBlueprintResources/StandardMacros.IsValid` _asbp_player
    (:`Is Valid`
      (cast `CapsuleComponent` OtherComp)
      (bind _charactermovement (`Character.CharacterMovement` _asbp_player))
      (`/Engine/EditorBlueprintResources/StandardMacros.IsValid` _charactermovement
        (:`Is Valid`
          (set `self.SpeedOriginal` (`MovementComponent.GetMaxSpeed` _charactermovement))
          (if (not (`/Game/BP/Player/BP_DashImpulseComponent.bIsDashing` (`/Game/BP/Player/BP_Player.BP_DashImpulseComponent` _asbp_player)))
            (`MovementComponent.StopMovementImmediately` _charactermovement))
          (set `CharacterMovementComponent.MaxWalkSpeed` (`self.SpeedMax`) _charactermovement))))))

(event `self.Box.OnComponentEndOverlap`
  (params (OverlappedComponent :type "PrimitiveComponent Object Reference") (OtherActor :type "Actor Object Reference") (OtherComp :type "PrimitiveComponent Object Reference") (OtherBodyIndex :type Integer))
  (bind _asbp_player (cast `/Game/BP/Player/BP_Player` OtherActor))
  (`/Engine/EditorBlueprintResources/StandardMacros.IsValid` _asbp_player
    (:`Is Valid`
      (bind _ascapsule_collision (cast `CapsuleComponent` OtherComp))
      (`/Engine/EditorBlueprintResources/StandardMacros.IsValid` _ascapsule_collision
        (:`Is Valid`
          (set `CharacterMovementComponent.MaxWalkSpeed` (`self.SpeedOriginal`) (`Character.CharacterMovement` _asbp_player)))))))

(fn `UserConstructionScript`
  (`parent.UserConstructionScript`))