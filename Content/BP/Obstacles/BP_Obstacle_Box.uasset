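; Explosive box obstacle that detonates when it hits the player, killing players in its blast radius and breaking step meshes.
; Each tick, a vertical line trace moves a Plane onto the surface hit, apparently as a ground marker.
; The explosion hides the box, spawns an effect actor and sphere-traces for victims, swapping specific step meshes to broken versions and destroying their attachments.
; The box then kills itself through its health component.
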(event `self.ReceiveTick`
  (params (DeltaSeconds :type "Float (single-precision)"))
  (bind _returnvalue (`self.K2_GetActorLocation`))
  (bind _outhit (`KismetSystemLibrary.LineTraceSingle` (+ _returnvalue (0.0 0.0 200.0)) (+ _returnvalue (0.0 0.0 -10000.0)) "TraceTypeQuery1"))
  (`SceneComponent.K2_SetWorldLocation` (`self.Plane`) (`.Location` (`GameplayStatics.BreakHitResult` _outhit)) false false))

(event `self.StaticMesh.OnComponentHit`
  (params (HitComponent :type "PrimitiveComponent Object Reference") (OtherActor :type "Actor Object Reference") (OtherComp :type "PrimitiveComponent Object Reference") (NormalImpulse :type "Vector Structure") (Hit :type "HitResult Structure (by ref)"))
  (cast `/Game/BP/Player/BP_Player` OtherActor)
  (`self.Explode`))

(event `Explode`
  (bind _returnvalue (`self.K2_GetActorLocation`))
  (`SceneComponent.SetVisibility` (`self.StaticMesh`) false false)
  (`|SpawnActorFromClass` "/Game/BP/Obstacles/BP_Explosion.BP_Explosion_C" (`KismetMathLibrary.MakeTransform` (`self.K2_GetActorLocation`) (struct) (2.0 2.0 2.0)) "Undefined" "OverrideRootScale" null null)
  (`PrimitiveComponent.SetCollisionEnabled` (`self.StaticMesh`) "NoCollision")
  (bind _outhits (`KismetSystemLibrary.SphereTraceMultiForObjects` _returnvalue _returnvalue (`self.ExplosionRadius`) (`self.Object Types`)))
  (for _array_element _outhits
    (bind _asbp_player (cast `/Game/BP/Player/BP_Player` (`.HitActor` (`GameplayStatics.BreakHitResult` _array_element)))
      (:`then`
        (`/Game/BP/ActorComponents/BPC_HealthComponent.KillActor` (`/Game/BP/Player/BP_Player.BPC_HealthComponent` _asbp_player) 3.0))
      (:`CastFailed`
        (bind _asstatic_mesh_actor (cast `StaticMeshActor` (`.HitActor` (`GameplayStatics.BreakHitResult` _array_element))))
        (if (== (`StaticMeshComponent.StaticMesh` (`StaticMeshActor.StaticMeshComponent` _asstatic_mesh_actor)) "/Game/Materials/SM_Step_Test_6.SM_Step_Test_6")
          (`StaticMeshComponent.SetStaticMesh` (`StaticMeshActor.StaticMeshComponent` _asstatic_mesh_actor) "/Game/Materials/SM_Step_Broken.SM_Step_Broken")
          (for _array_element_2 (`self.GetAttachedActors` _asstatic_mesh_actor true)
            (`self.K2_DestroyActor` _array_element_2))))))
  (`/Game/BP/ActorComponents/BPC_HealthComponent.KillActor` (`self.BPC_HealthComponent`) 0.5))

(fn `UserConstructionScript`
  (`parent.UserConstructionScript`))